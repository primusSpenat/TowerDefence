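; BP_Ammo_Projectile is a tower-fired splash projectile that travels in an arc from its start location to a set impact point.
; A timeline, rate-scaled by projectile speed over distance, moves it along the horizontal path while a separate Z track shapes the height.
; When the timeline finishes, it spawns an emitter and sphere-traces the splash radius, applying flat damage to enemies with the owning tower as causer.
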(event Custom|OnExplode
  (bind _impactlocation (Variables|Default|GetImpactLocation))
  (Effects|SpawnEmitteratLocation 0 (Variables|Default|GetImpactLocation))
  (bind (_outhits _returnvalue) (Collision|MultiSphereTraceForObjects _impactlocation (- _impactlocation "0, 0,-1.000000") (Variables|Default|GetSplashRadius) (Utilities|Array|MakeArray "ObjectTypeQuery7") false 0 "None"))
  (if _returnvalue
    (for _array_element _outhits
      (Utilities|Casting|CastToBP_Enemy (.HitActor (Collision|BreakHitResult _array_element)))
      (Game|Damage|ApplyDamage 0 (Variables|Default|GetSplashDamage) 0 (Variables|Default|GetOwningTower)))))

(event EventBeginPlay
  (Components|Sphere|SetSphereRadius (Variables|Default|GetSphere) (Variables|Default|GetSplashRadius) false)
  (Components|Timeline|SetPlayRate (Variables|Default|GetTravelTimeline) (/ (Variables|Default|GetProjectileSpeed) (Math|Vector|VectorLength (- (Variables|Default|GetStartLocation) (Variables|Default|GetImpactLocation)))))
  (bind (_direction _travelcurve _z_trajectory) (Timeline|TravelTimeline PlayFromStart)
    (:Update
      (Transformation|SetActorLocation (Math|Vector|MakeVector (.X (Math|Vector|BreakVector (Math|Vector|Lerp(Vector) (Variables|Default|GetStartLocation) (Variables|Default|GetImpactLocation) _travelcurve))) (.Y (Math|Vector|BreakVector (Math|Vector|Lerp(Vector) (Variables|Default|GetStartLocation) (Variables|Default|GetImpactLocation) _travelcurve))) (Math|Float|Lerp _z_trajectory (+ (Math|Float|Lerp (.Z (Math|Vector|BreakVector (Variables|Default|GetStartLocation))) (.Z (Math|Vector|BreakVector (Variables|Default|GetImpactLocation))) _z_trajectory) (Variables|Default|GetTrajectoryZValue)) _z_trajectory)) false false))
    (:Finished
      (CallFunction|OnExplode))))

(fn ConstructionScript)