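; Master tower actor for a tower defense game that automatically targets and shoots enemies in range.
; BeginPlay loads the hardcoded "Hitscan" DT_Tower row, which sets mesh, range sphere, effects and the DT_Ammo lookup.
; Range overlaps drive targeting, favoring the enemy nearest the spawn manager's EndLocation.
; Shots spawn hitscan ammo or a projectile aimed at ground traced beneath the target, then re-acquire after the fire-rate delay.
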(event OnComponentBeginOverlap(TowerTriggerRange)
  (params (OverlappedComponent :type Primitive%20Component%20Object%20Reference) (OtherActor :type Actor%20Object%20Reference) (OtherComp :type Primitive%20Component%20Object%20Reference) (OtherBodyIndex :type Integer) (bFromSweep :type Boolean) (SweepResult :type Hit%20Result%20Structure%20%28by%20ref%29))
  (Variables|Default|GetTowerTarget
    (:then)
    (:else
      (bind _asbp_enemy (Utilities|Casting|CastToBP_Enemy OtherActor))
      (Utilities|FlowControl|Sequence
        (:then_0
          (Utilities|FlowControl|DoOnce false
            (:Completed
              (Variables|Default|SetTowerTarget _asbp_enemy))))
        (:then_1
          _))
      (Variables|Default|SetbShouldLookForTargets true)
      (CallFunction|OnLookforTargets))))

(event OnComponentEndOverlap(TowerTriggerRange)
  (params (OverlappedComponent :type Primitive%20Component%20Object%20Reference) (OtherActor :type Actor%20Object%20Reference) (OtherComp :type Primitive%20Component%20Object%20Reference) (OtherBodyIndex :type Integer))
  (if (== OtherActor (Variables|Default|GetTowerTarget))
    (Variables|Default|SetTowerTarget 0)))

(event Custom|OnTowerInit
  (bind _towerstructreff (Variables|Default|GetTowerStructReff))
  (|SetStructReff (.name _towerstructreff) (.damage _towerstructreff) (.range _towerstructreff) (.firerate _towerstructreff) (.cost _towerstructreff) (.bshouldrotate _towerstructreff) (.attacktype _towerstructreff) (.bhassplashdamage _towerstructreff) (.splashradius _towerstructreff) (.splashdamage _towerstructreff) (.projectilereference _towerstructreff) (.shootingsound _towerstructreff) (.impactsound _towerstructreff) (.shootingparticle _towerstructreff) (.staticmesh _towerstructreff)))

(event Custom|OnLookForTargets
  (bind _towertriggerrange (Variables|Default|GetTowerTriggerRange))
  (bind _overlappingactors (Collision|GetOverlappingActors _towertriggerrange "/Game/Core/AI/BP_Enemy.BP_Enemy_C" :!class /Script/Engine.PrimitiveComponent))
  (Utilities|IsValid (Variables|Default|GetTowerTarget)
    (:Is%20Valid
      (if (Variables|Default|GetbShooting)
        (Utilities|FlowControl|Delay 0.2)
        (CallFunction|OnLookforTargets)
        (else
          (CallFunction|OnShooting))))
    (:Is%20Not%20Valid
      (if (Variables|Default|GetbShouldLookForTargets)
        (Variables|Default|SetbShouldLookForTargets false)
        (Variables|Default|SetOverlappingTargets _overlappingactors)
        (if (== (Utilities|Array|Length _overlappingactors) 0)
          (CallFunction|OnNoOverlappingEnemies)
          (else
            (bind _finaltarget (CallFunction|GetClosestTarget _overlappingactors))
            (bind _asbp_enemy (Utilities|Casting|CastToBP_Enemy _finaltarget))
            (Variables|Default|SetTowerTarget _asbp_enemy)
            (Variables|Default|SetbShouldLookForTargets true)
            (CallFunction|OnLookforTargets)))))))

(event Custom|OnShooting
  (bind _towermesh (Variables|Default|GetTowerMesh))
  (bind _returnvalue (Transformation|GetSocketLocation _towermesh "ShootingSocket"))
  (Variables|Default|SetbShooting true)
  ;[1 0.05048 0] DEBUG LINE
  (Rendering|Debug|DrawDebugLine (Transformation|GetSocketLocation (Variables|Default|GetTowerMesh) "ShootingSocket") (Transformation|GetActorLocation (Variables|Default|GetTowerTarget)) "(R=1.000000,G=0.216922,B=0.107200,A=1.000000)" 0.2 4.0)
  (Effects|SpawnEmitteratLocation (Variables|Default|GetTowerShootingParticleReff) _returnvalue)
  (Audio|PlaySoundatLocation (Variables|Default|GetTowerShootingSoundReff) _returnvalue "0, 0, 0" 1.0 1.0 0.0 0 0 0)
  (switch Utilities|FlowControl|Switch|SwitchonE_AttackType (Variables|Default|GetTowerAttackTypeReff)
    (:NewEnumerator0
      (|HitScanLogicGraph))
    (:NewEnumerator1
      (|ProjectileLogicGraph))))

(event Custom|OnFireRateDelay
  (Utilities|FlowControl|Delay (Variables|Default|GetTowerFireRateReff))
  (Variables|Default|SetbShooting false)
  (CallFunction|OnLookforTargets))

(event Custom|OnNoOverlappingEnemies
  (Utilities|FlowControl|DoOnce false) ; enters at Reset
)

(event EventBeginPlay
  (bind _outactors (Actor|GetAllActorsOfClass "/Game/Core/AI/BP_EnemySpawnManager.BP_EnemySpawnManager_C"))
  (Variables|Default|SetSpawnManagerReff (Utilities|Array|Get(acopy) _outactors))
  (bind _returnvalue (Utilities|GetDataTableRow "/Game/Core/Tower/DT_Tower.DT_Tower" "Hitscan")
    (:then
      (Utilities|FlowControl|Delay 0.2)
      (Variables|Default|SetTowerStructReff _returnvalue)
      (CallFunction|OnTowerInit))))

(fn ConstructionScript)

(fn GetClosestTarget
  (params (DetectedEnemies :type Array%20of%20Actor%20Object%20References))
  (LocalVariables|SetMyTempDistance (Variables|Default|GetTowerRangeReff))
  (for _array_element DetectedEnemies
    (LocalVariables|GetMyTempTarget
      (:then
        (if (< (Math|Vector|VectorLength (- (Variables|/Game/Core/AI/BP_EnemySpawnManager.BP_EnemySpawnManager_C|GetEndLocation (Variables|Default|GetSpawnManagerReff)) (Transformation|GetActorLocation _array_element))) (LocalVariables|GetMyTempDistance))
          (LocalVariables|SetMyTempTarget _array_element)
          (LocalVariables|SetMyTempDistance (Math|Vector|VectorLength (- (Variables|/Game/Core/AI/BP_EnemySpawnManager.BP_EnemySpawnManager_C|GetEndLocation (Variables|Default|GetSpawnManagerReff)) (Transformation|GetActorLocation _array_element))))))
      (:else
        (LocalVariables|SetMyTempTarget _array_element)
        (LocalVariables|SetMyTempDistance (Math|Vector|VectorLength (- (Variables|/Game/Core/AI/BP_EnemySpawnManager.BP_EnemySpawnManager_C|GetEndLocation (Variables|Default|GetSpawnManagerReff)) (Transformation|GetActorLocation _array_element)))))))
  (return (LocalVariables|GetMyTempTarget)))