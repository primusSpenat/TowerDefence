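; Tower defense spawn manager that runs data-driven enemy waves and deducts a player life when an enemy reaches its finish line trigger.
; After game mode clearance it caches the wave table, registers with the HUD and shows the next-wave widget.
; Rows define timed groups or wave breaks, walked by a delay-driven loop.
; A single BP_Enemy class spawns at chosen or random offsets, configured from DT_Enemy by type.
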(event OnComponentBeginOverlap(FinishLineTrigger)
  (params (OverlappedComponent :type Primitive%20Component%20Object%20Reference) (OtherActor :type Actor%20Object%20Reference) (OtherComp :type Primitive%20Component%20Object%20Reference) (OtherBodyIndex :type Integer) (bFromSweep :type Boolean) (SweepResult :type Hit%20Result%20Structure%20%28by%20ref%29))
  (Utilities|Casting|CastToBP_Enemy OtherActor)
  (bind _astd_playerstate (Utilities|Casting|CastToTD_Playerstate (Variables|/Script/Engine.Controller|GetPlayerState (Game|GetPlayerController 0))))
  (Default|OnUpdatePlayerLives _astd_playerstate -1)
  (bind _astd_gamestate (Utilities|Casting|CastToTD_Gamestate (Game|GetGameState)))
  (Default|OnRemoveandCheckEnemiesRemaining _astd_gamestate)
  (Actor|DestroyActor OtherActor))

(event Custom|OnStartNextWave
  (if (> (Utilities|Array|Length (Variables|Default|GetAIWaveDTRows)) (Variables|Default|GetCurrentWaveDTIndex))
    (bind _returnvalue (Utilities|GetDataTableRow (Variables|Default|GetEnemyWaveDTReff) (Utilities|Array|Get(acopy) (Variables|Default|GetAIWaveDTRows) (Variables|Default|GetCurrentWaveDTIndex)))
      (:then
        (bind _output_get (Variables|Default|SetEnemyWaveStructReff _returnvalue))
        (switch Utilities|FlowControl|Switch|SwitchonE_Types (.type _output_get)
          (:NewEnumerator0
            (bind _returnvalue_2 (Utilities|GetDataTableRow "/Game/Core/AI/DT_Enemy.DT_Enemy" "Small")
              (:then
                (CallFunction|MyMakeEnemy _returnvalue_2))))
          (:NewEnumerator1
            (bind _returnvalue_3 (Utilities|GetDataTableRow "/Game/Core/AI/DT_Enemy.DT_Enemy" "Mech")
              (:then
                (CallFunction|MyMakeEnemy _returnvalue_3))))
          (:NewEnumerator2
            (bind _returnvalue_4 (Utilities|GetDataTableRow "/Game/Core/AI/DT_Enemy.DT_Enemy" "Flying")
              (:then
                (CallFunction|MyMakeEnemy _returnvalue_4))))
          (:NewEnumerator3
            (Math|Integer|IncrementInt (Variables|Default|GetCurrentWaveDTIndex)
              (:%20%20
                (Math|Integer|IncrementInt (Variables|Default|GetCurrentWaveNumber)
                  (:%20%20
                    (if (!= (Utilities|Array|Length (Variables|Default|GetAIWaveDTRows)) (Variables|Default|GetCurrentWaveDTIndex))
                      (Default|OnCreateNextWaveWidget (Variables|Default|GetHUDReff) (Variables|Default|GetCurrentWaveNumber))))))))))
      (:RowNotFound
        (Development|PrintString "No Row")))
    (else
      (Development|PrintString "No more waves!" true true "(R=0.222475,G=1.000000,B=0.142221,A=1.000000)" 5.0))))

(event Custom|OnLoopEnemySpawnAmount
  (bind _enemywavestructreff (Variables|Default|GetEnemyWaveStructReff))
  (Utilities|FlowControl|Delay (.timebetweenenemy _enemywavestructreff))
  (if (== (.numberofenemies _enemywavestructreff) (Variables|Default|GetEnemyCounter))
    (Variables|Default|SetEnemyCounter 0)
    (Utilities|FlowControl|Delay (.timetonextgroup (Variables|Default|GetEnemyWaveStructReff)))
    (Math|Integer|IncrementInt (Variables|Default|GetCurrentWaveDTIndex)
      (:%20%20
        (CallFunction|OnStartNextWave)))
    (else
      (switch Utilities|FlowControl|Switch|SwitchonE_Types (.type (stale Custom|OnStartNextWave _output_get))
        (:NewEnumerator0
          (bind _returnvalue (Utilities|GetDataTableRow "/Game/Core/AI/DT_Enemy.DT_Enemy" "Small")
            (:then
              (CallFunction|MyMakeEnemy _returnvalue))))
        (:NewEnumerator1
          (bind _returnvalue_2 (Utilities|GetDataTableRow "/Game/Core/AI/DT_Enemy.DT_Enemy" "Mech")
            (:then
              (CallFunction|MyMakeEnemy _returnvalue_2))))
        (:NewEnumerator2
          (bind _returnvalue_3 (Utilities|GetDataTableRow "/Game/Core/AI/DT_Enemy.DT_Enemy" "Flying")
            (:then
              (CallFunction|MyMakeEnemy _returnvalue_3))))
        (:NewEnumerator3
          (Math|Integer|IncrementInt (Variables|Default|GetCurrentWaveDTIndex)
            (:%20%20
              (Math|Integer|IncrementInt (Variables|Default|GetCurrentWaveNumber)
                (:%20%20
                  (if (!= (Utilities|Array|Length (Variables|Default|GetAIWaveDTRows)) (Variables|Default|GetCurrentWaveDTIndex))
                    (Default|OnCreateNextWaveWidget (Variables|Default|GetHUDReff) (Variables|Default|GetCurrentWaveNumber))))))))))))

(event Custom|OnWaitForGamemodeClearance
  (Utilities|FlowControl|Sequence
    (:then_0
      (bind _astd_hud (Utilities|Casting|CastToTD_Hud (HUD|GetHUD (Game|GetPlayerController 0))))
      (Variables|Default|SetHUDReff _astd_hud)
      (Variables|/Game/Core/TD_Hud.TD_Hud_C|SetSpawnManagerReff _astd_hud self))
    (:then_1
      (Default|OnCreateNextWaveWidget (Variables|Default|GetHUDReff) (Variables|Default|GetCurrentWaveNumber)))
    (:then_2
      (bind _astd_game_mode (Utilities|Casting|CastToTD_GameMode (Game|GetGameMode)))
      (Variables|Default|SetEnemyWaveDTReff (Variables|/Game/Core/TD_GameMode.TD_GameMode_C|GetEnemyWaveDT _astd_game_mode))
      (Variables|Default|SetAIWaveDTRows (Variables|/Game/Core/TD_GameMode.TD_GameMode_C|GetEnemyWaveDTRowNames _astd_game_mode)))))

(event EventBeginPlay
  (bind _astd_game_mode (Utilities|Casting|CastToTD_GameMode (Game|GetGameMode)))
  (bind _output_get (Variables|Default|SetGameModeReff _astd_game_mode))
  (EventDispatchers|BindEventtoEDGamemodeComplete _output_get (delegate Custom|OnWaitForGamemodeClearance)))

(fn ConstructionScript)

(fn MyMakeEnemy
  (params (EnemyStruct :type S%20Enemy%20Structure))
  (bind _spawnlocation01 (Variables|Default|GetSpawnLocation01))
  (bind _spawnlocation02 (Variables|Default|GetSpawnLocation02))
  (bind _spawnlocation03 (Variables|Default|GetSpawnLocation03))
  (bind _array (Utilities|Array|MakeArray _spawnlocation01 _spawnlocation02 _spawnlocation03))
  (Variables|Default|SetEnemyStructReff EnemyStruct)
  (Utilities|FlowControl|Sequence
    (:then_0
      (switch Utilities|FlowControl|Switch|SwitchonE_SpawnLocations (.spawnlocation (Variables|Default|GetEnemyWaveStructReff))
        (:NewEnumerator3
          (bind _returnvalue (AI|SpawnAIFromClass "/Game/Core/AI/BP_Enemy.BP_Enemy_C" "/Game/Core/AI/BT_Enemy.BT_Enemy" (+ (Utilities|Array|Get(acopy) _array (Math|Random|RandomIntegerinRange 0 (- (Utilities|Array|Length _array) 1))) (Transformation|GetActorLocation)) "0, 0, 0" true))
          (bind _asbp_enemy (Utilities|Casting|CastToBP_Enemy _returnvalue))
          (Variables|Default|SetEnemyReff _asbp_enemy)
          (bind _asbp_enemy_controller (Utilities|Casting|CastToBP_EnemyController (Pawn|GetController _asbp_enemy)))
          (Variables|/Game/Core/AI/BP_EnemyController.BP_EnemyController_C|SetSpawnManagerReff _asbp_enemy_controller self)
          (Math|Integer|IncrementInt (Variables|Default|GetEnemyCounter)))
        (:NewEnumerator0
          (bind _returnvalue_2 (AI|SpawnAIFromClass "/Game/Core/AI/BP_Enemy.BP_Enemy_C" "/Game/Core/AI/BT_Enemy.BT_Enemy" (+ (Variables|Default|GetSpawnLocation01) (Transformation|GetActorLocation)) "0, 0, 0" true))
          (bind _asbp_enemy_2 (Utilities|Casting|CastToBP_Enemy _returnvalue_2))
          (Variables|Default|SetEnemyReff _asbp_enemy_2)
          (bind _asbp_enemy_controller_2 (Utilities|Casting|CastToBP_EnemyController (Pawn|GetController _asbp_enemy_2)))
          (Variables|/Game/Core/AI/BP_EnemyController.BP_EnemyController_C|SetSpawnManagerReff _asbp_enemy_controller_2 self)
          (Math|Integer|IncrementInt (Variables|Default|GetEnemyCounter)))
        (:NewEnumerator1
          (bind _returnvalue_3 (AI|SpawnAIFromClass "/Game/Core/AI/BP_Enemy.BP_Enemy_C" "/Game/Core/AI/BT_Enemy.BT_Enemy" (+ (Variables|Default|GetSpawnLocation02) (Transformation|GetActorLocation)) "0, 0, 0" true))
          (bind _asbp_enemy_3 (Utilities|Casting|CastToBP_Enemy _returnvalue_3))
          (Variables|Default|SetEnemyReff _asbp_enemy_3)
          (bind _asbp_enemy_controller_3 (Utilities|Casting|CastToBP_EnemyController (Pawn|GetController _asbp_enemy_3)))
          (Variables|/Game/Core/AI/BP_EnemyController.BP_EnemyController_C|SetSpawnManagerReff _asbp_enemy_controller_3 self)
          (Math|Integer|IncrementInt (Variables|Default|GetEnemyCounter)))
        (:NewEnumerator2
          (bind _returnvalue_4 (AI|SpawnAIFromClass "/Game/Core/AI/BP_Enemy.BP_Enemy_C" "/Game/Core/AI/BT_Enemy.BT_Enemy" (+ (Variables|Default|GetSpawnLocation03) (Transformation|GetActorLocation)) "0, 0, 0" true))
          (bind _asbp_enemy_4 (Utilities|Casting|CastToBP_Enemy _returnvalue_4))
          (Variables|Default|SetEnemyReff _asbp_enemy_4)
          (bind _asbp_enemy_controller_4 (Utilities|Casting|CastToBP_EnemyController (Pawn|GetController _asbp_enemy_4)))
          (Variables|/Game/Core/AI/BP_EnemyController.BP_EnemyController_C|SetSpawnManagerReff _asbp_enemy_controller_4 self)
          (Math|Integer|IncrementInt (Variables|Default|GetEnemyCounter)))))
    (:then_1
      (Components|StaticMesh|SetStaticMesh (Variables|/Game/Core/AI/BP_Enemy.BP_Enemy_C|GetStaticMesh (Variables|Default|GetEnemyReff)) (.mesh (Variables|Default|GetEnemyStructReff)))
      (Variables|/Script/Engine.CharacterMovementComponent|SetMaxWalkSpeed (Variables|/Script/Engine.Character|GetCharacterMovement (Variables|Default|GetEnemyReff)) (.speed (Variables|Default|GetEnemyStructReff)))
      (Variables|/Game/Core/AI/BP_Enemy.BP_Enemy_C|SetHitpoints (Variables|Default|GetEnemyReff) (.hitpoint (Variables|Default|GetEnemyStructReff)))
      (Variables|/Game/Core/AI/BP_Enemy.BP_Enemy_C|SetReward (Variables|Default|GetEnemyReff) (.reward (Variables|Default|GetEnemyStructReff))))
    (:then_2
      (CallFunction|OnLoopEnemySpawnAmount))))